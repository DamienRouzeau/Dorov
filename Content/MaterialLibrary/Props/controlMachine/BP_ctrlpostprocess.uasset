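; BP_ctrlpostprocess is an interactive control-box prop with screens, animated controls and four status diodes.
; Events play arrow, button and joystick animations, with resettable DoOnce gates and anim pausing managing joystick poses.
; changeProps forwards an index to the image and text-list widgets, while ChangeDiode swaps a diode's material between green and red.
; A sphere overlap toggles custom depth on the box mesh while the first-person character is in range.
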(event `changeProps`
  (params (index :type Integer))
  (bind _asui_screen (cast `/Game/UI/uiCtrlBox/UI_Screen` (`WidgetComponent.GetUserWidgetObject` (`self.screen`))))
  (`/Game/UI/uiCtrlBox/UI_Screen.changeImage` _asui_screen index)
  (bind _asui_text_list (cast `/Game/UI/uiCtrlBox/UI_TextList` (`WidgetComponent.GetUserWidgetObject` (`self.TextScreen`))))
  (`/Game/UI/uiCtrlBox/UI_TextList.changeProps` _asui_text_list index))

(event `LeftArrow`
  (`self.UnPause`)
  (`SkeletalMeshComponent.PlayAnimation` (`self.Ctrl_Box_SkelMesh`) "/Game/BlockOut_Theatres/CtrlBox/ANIMs/A_Ctrl_box_Arrow_L.A_Ctrl_box_Arrow_L" false))

(event `RightArrow`
  (`self.UnPause`)
  (`SkeletalMeshComponent.PlayAnimation` (`self.Ctrl_Box_SkelMesh`) "/Game/BlockOut_Theatres/CtrlBox/ANIMs/A_Ctrl_box_Arrow_R.A_Ctrl_box_Arrow_R" false))

(event `ConfirmBtn`
  (`self.UnPause`)
  (`SkeletalMeshComponent.PlayAnimation` (`self.Ctrl_Box_SkelMesh`) "/Game/BlockOut_Theatres/CtrlBox/ANIMs/A_Ctrl_box_Button.A_Ctrl_box_Button" false))

(event `JoyRight`
  (bind _ctrl_box_skelmesh (`self.Ctrl_Box_SkelMesh`))
  (bind _ctrl_box_skelmesh_2 (`self.Ctrl_Box_SkelMesh`))
  (`/Engine/EditorBlueprintResources/StandardMacros.DoOnce` false :!label _label
    (:`Completed`
      (`self.UnPause`)
      (`SkeletalMeshComponent.PlayAnimation` _ctrl_box_skelmesh_2 "/Game/BlockOut_Theatres/CtrlBox/ANIMs/A_Ctrl_box_Joystick_R.A_Ctrl_box_Joystick_R" true)
      (`KismetSystemLibrary.Delay` 0.5)
      (set `SkeletalMeshComponent.bPauseAnims` true _ctrl_box_skelmesh_2)
      (`|ExecutionSequence`
        (:`then_0`
          (goto _label_2 :!via `Reset`))
        (:`then_1`
          (goto _label_3 :!via `Reset`))))))

(event `JoyLeft`
  (bind _ctrl_box_skelmesh (`self.Ctrl_Box_SkelMesh`))
  (bind _ctrl_box_skelmesh_2 (`self.Ctrl_Box_SkelMesh`))
  (`/Engine/EditorBlueprintResources/StandardMacros.DoOnce` false :!label _label_2
    (:`Completed`
      (`self.UnPause`)
      (`SkeletalMeshComponent.PlayAnimation` _ctrl_box_skelmesh_2 "/Game/BlockOut_Theatres/CtrlBox/ANIMs/A_Ctrl_box_Joystick_L.A_Ctrl_box_Joystick_L" true)
      (`KismetSystemLibrary.Delay` 0.5)
      (set `SkeletalMeshComponent.bPauseAnims` true _ctrl_box_skelmesh_2)
      (`|ExecutionSequence`
        (:`then_0`
          (goto _label :!via `Reset`))
        (:`then_1`
          (goto _label_3 :!via `Reset`))))))

(event `JoyIdle`
  (bind _ctrl_box_skelmesh (`self.Ctrl_Box_SkelMesh`))
  (`/Engine/EditorBlueprintResources/StandardMacros.DoOnce` false :!label _label_3
    (:`Completed`
      (`self.UnPause`)
      (`SkeletalMeshComponent.PlayAnimation` _ctrl_box_skelmesh "/Game/BlockOut_Theatres/CtrlBox/ANIMs/A_Ctrl_box_Joystick_T.A_Ctrl_box_Joystick_T" true)
      (set `SkeletalMeshComponent.bPauseAnims` true _ctrl_box_skelmesh)
      (`|ExecutionSequence`
        (:`then_0`
          (goto _label :!via `Reset`))
        (:`then_1`
          (goto _label_2 :!via `Reset`))))))

(event `self.Sphere.OnComponentBeginOverlap`
  (params (OverlappedComponent :type "PrimitiveComponent Object Reference") (OtherActor :type "Actor Object Reference") (OtherComp :type "PrimitiveComponent Object Reference") (OtherBodyIndex :type Integer) (bFromSweep :type Boolean) (SweepResult :type "HitResult Structure (by ref)"))
  (cast `/Game/FirstPerson/Blueprints/BP_FirstPersonCharacter` OtherActor)
  (`PrimitiveComponent.SetRenderCustomDepth` (`self.Ctrl_Box_SkelMesh`) true))

(event `self.Sphere.OnComponentEndOverlap`
  (params (OverlappedComponent :type "PrimitiveComponent Object Reference") (OtherActor :type "Actor Object Reference") (OtherComp :type "PrimitiveComponent Object Reference") (OtherBodyIndex :type Integer))
  (cast `/Game/FirstPerson/Blueprints/BP_FirstPersonCharacter` OtherActor)
  (`PrimitiveComponent.SetRenderCustomDepth` (`self.Ctrl_Box_SkelMesh`) false))

(event `ChangeDiode`
  (params (DiodeToChange :type Integer) (TurnToGreen :type Boolean))
  (if TurnToGreen
    (set `self.CurrentDiode` (`self.GreenDiode`))
    (else
      (set `self.CurrentDiode` (`self.RedDiode`))))
  (if (== DiodeToChange 1)
    (`PrimitiveComponent.SetMaterial` (`self.S1Diode`) 0 (`self.CurrentDiode`))
    (elif (== DiodeToChange 2)
      (`PrimitiveComponent.SetMaterial` (`self.S2Diode`) 0 (`self.CurrentDiode`))
      (elif (== DiodeToChange 3)
        (`PrimitiveComponent.SetMaterial` (`self.S3Diode`) 0 (`self.CurrentDiode`))
        (elif (== DiodeToChange 4)
          (`PrimitiveComponent.SetMaterial` (`self.S4Diode`) 0 (`self.CurrentDiode`)))))))

(fn `UnPause`
  (set `SkeletalMeshComponent.bPauseAnims` false (`self.Ctrl_Box_SkelMesh`)))

(fn `UserConstructionScript`)