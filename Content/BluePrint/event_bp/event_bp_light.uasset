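; An event Blueprint that switches off the level's normal and buzzing lights when any actor begins overlapping it.
; On overlap it gathers every Light_normal and Buzing_light actor into arrays and loops over each.
; Normal lights have their SpotLight intensity set to zero, while buzzing lights have their SpotLight hidden.
; The overlap has no actor filter or one-shot guard, and nothing here turns the lights back on.
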(event `self.ReceiveActorBeginOverlap`
  (params (OtherActor :type "Actor Object Reference"))
  (bind _liste_lightbuzzing (`self.liste_lightbuzzing`))
  (bind _light_normal (`self.light_normal`))
  (bind _outactors (`GameplayStatics.GetAllActorsOfClass` "/Game/BluePrint/lamp/buzing_light.buzing_light_C"))
  (set `self.liste_lightbuzzing` _outactors)
  (bind _outactors_2 (`GameplayStatics.GetAllActorsOfClass` "/Game/BluePrint/lamp/light_normal.light_normal_C"))
  (set `self.light_normal` _outactors_2)
  (for _index (range (+ (`KismetArrayLibrary.Array_LastIndex` _light_normal) 1))
    (`LightComponent.SetIntensity` (`/Game/BluePrint/lamp/light_normal.SpotLight` (`|GetArrayItem` _light_normal _index)) 0.0))
  (for _index_2 (range (+ (`KismetArrayLibrary.Array_LastIndex` _liste_lightbuzzing) 1))
    (`SceneComponent.SetVisibility` (`/Game/BluePrint/lamp/buzing_light.SpotLight` (`|GetArrayItem` _liste_lightbuzzing _index_2)) false false)))

(fn `UserConstructionScript`)