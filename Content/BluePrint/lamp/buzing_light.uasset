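; Lamp Blueprint that makes a spot light flicker like a buzzing, faulty bulb.
; Tick waits a random few seconds, then calls the Buzzz event, which briefly dims and restores the SpotLight intensity.
; Buzzz re-calls itself after short delays until Count reaches BuzCount, then resets the counter for the next burst.
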(event `self.ReceiveTick`
  (params (DeltaSeconds :type "Float (single-precision)"))
  (`KismetSystemLibrary.Delay` (`KismetMathLibrary.RandomFloatInRange` 2.0 6.0))
  (`self.buzzz`))

(event `buzzz`
  (bind _spotlight (`self.SpotLight`))
  (if (< (`self.count`) (`self.buz_count`))
    (`LightComponent.SetIntensity` _spotlight 3000.0)
    (`KismetSystemLibrary.Delay` 0.05)
    (`LightComponent.SetIntensity` _spotlight 7500.0)
    (set `self.count` (+ (`self.count`) 1))
    (`KismetSystemLibrary.Delay` 0.05)
    (`self.buzzz`)
    (else
      (set `self.count` 0))))

(fn `UserConstructionScript`)