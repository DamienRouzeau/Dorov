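; BP_Closet is a locker with an animated door that swings open and shuts by itself, plus a switchable point light.
; Tick eases the door's relative rotation toward an open yaw or the closed rotation cached at BeginPlay, using a fixed-alpha lerp.
; OpenAnimation, GetingOut and OpenAnimationLocker set the Open flag and reset a DoOnce, which arms a short timer that clears the flag.
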(event `self.ReceiveBeginPlay`
  (set `self.CloseRotation` (`SceneComponent.RelativeRotation` (`self.Casier_01_Porte_Casier_01`))))

(event `ResetOpen`
  (goto _label :!via `Reset`))

(event `CloseDoor`
  (set `self.open` false))

(event `TurnOnLight`
  (`SceneComponent.SetVisibility` (`self.PointLight`) true false))

(event `self.ReceiveTick`
  (params (DeltaSeconds :type "Float (single-precision)"))
  (bind _casier_01_porte_casier_01 (`self.Casier_01_Porte_Casier_01`))
  (bind _casier_01_porte_casier_01_2 (`self.Casier_01_Porte_Casier_01`))
  (bind (_relativerotation_roll _relativerotation_pitch) (`KismetMathLibrary.BreakRotator` (`SceneComponent.RelativeRotation` _casier_01_porte_casier_01)))
  (if (`self.open`)
    (`SceneComponent.K2_SetRelativeRotation` _casier_01_porte_casier_01 (`KismetMathLibrary.RLerp` (`SceneComponent.RelativeRotation` _casier_01_porte_casier_01) (`KismetMathLibrary.MakeRotator` _relativerotation_roll _relativerotation_pitch -120.0) 0.3) false false)
    (`/Engine/EditorBlueprintResources/StandardMacros.DoOnce` false :!label _label
      (:`Completed`
        (`KismetSystemLibrary.K2_SetTimerDelegate` (delegate `CloseDoor`) 0.4)))
    (else
      (`SceneComponent.K2_SetRelativeRotation` _casier_01_porte_casier_01_2 (`KismetMathLibrary.RLerp` (`SceneComponent.RelativeRotation` _casier_01_porte_casier_01_2) (`self.CloseRotation`) 0.3) false false))))

(event `TurnOffLight`
  (`SceneComponent.SetVisibility` (`self.PointLight`) false false))

(event `OpenAnimation`
  (set `self.open` true :!label _label_2)
  (`self.ResetOpen`))

(event `GetingOut`
  (goto _label_2))

(fn `OpenAnimationLocker`
  (returns (Camera :type "CameraComponent Object Reference"))
  (set `self.open` true)
  (`self.ResetOpen`)
  (return null))

(fn `UserConstructionScript`)