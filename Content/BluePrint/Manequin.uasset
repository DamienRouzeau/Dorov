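; Mannequin enemy that chases the first-person player, or heads for a Cible target actor while the player hides in a closet.
; While CanWalk is set, Tick reissues AI MoveTo, with a Delay pacing random-pitched, spatialized footstep sounds.
; Overlapping the player marks them Dead and opens the LobbyTheaterv2 level, while overlapping a Cible destroys the mannequin.
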(event `self.ReceiveTick`
  (params (DeltaSeconds :type "Float (single-precision)"))
  (if (`self.can_walk`)
    (bind _returnvalue (`GameplayStatics.GetActorOfClass` "/Game/FirstPerson/Blueprints/BP_FirstPersonCharacter.BP_FirstPersonCharacter_C"))
    (if (`/Game/FirstPerson/Blueprints/BP_FirstPersonCharacter.IsInCloset` _returnvalue)
      (bind _returnvalue_2 (`GameplayStatics.GetActorOfClass` "/Game/BluePrint/cible.cible_C"))
      (`|AIMoveTo` self (0.0 0.0 0.0) _returnvalue_2 20.0
        (:`then`
          _))
      (else
        (`|AIMoveTo` self (0.0 0.0 0.0) _returnvalue 10.0
          (:`then`
            _))))
    (`KismetSystemLibrary.Delay` 0.4)
    (`GameplayStatics.PlaySoundAtLocation` "/Game/sound/footsteps/348355__natty23__footstep.348355__natty23__footstep" (`self.K2_GetActorLocation`) (struct) 1.0 (`KismetMathLibrary.RandomFloatInRange` 0.1 2.0) 0.0 "/Game/sound/footsteps/NewSoundAttenuation.NewSoundAttenuation" null null null)))

(event `self.ReceiveActorBeginOverlap`
  (params (OtherActor :type "Actor Object Reference"))
  (if (== (`GameplayStatics.GetObjectClass` OtherActor) "/Game/FirstPerson/Blueprints/BP_FirstPersonCharacter.BP_FirstPersonCharacter_C")
    (bind _asbp_first_person_character (cast `/Game/FirstPerson/Blueprints/BP_FirstPersonCharacter` OtherActor))
    (set `/Game/FirstPerson/Blueprints/BP_FirstPersonCharacter.dead` true _asbp_first_person_character)
    (`GameplayStatics.OpenLevelBySoftObjectPtr` "/Game/Maps/LobbyTheaterv2.LobbyTheaterv2")
    (else
      (cast `/Game/BluePrint/cible` OtherActor)
      (`self.K2_DestroyActor`))))

(fn `UserConstructionScript`)