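; AI controller for the Weeping Angel enemy, which chases the player only while they are not looking at it.
; Each tick, once the angel has detected the player and is over 300 units away, it compares the camera's forward vector with the angel-to-camera direction via a dot product.
; When unwatched, the angel turns its yaw toward the player and moves to them; when watched, it stops.
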(event `self.ReceiveBeginPlay`)

(event `self.ReceiveTick`
  (params (DeltaSeconds :type "Float (single-precision)"))
  (bind _asbp_weeping_angel (cast `/Game/weepingAngel/Blueprint/BP_WeepingAngel` (`self.K2_GetPawn`)))
  (if (`/Game/weepingAngel/Blueprint/BP_WeepingAngel.isPlayerDetected` _asbp_weeping_angel)
    (if (> (`self.GetDistanceTo` (`GameplayStatics.GetPlayerCharacter` 0) (`self.K2_GetPawn`)) 300.0)
      (`self.DetectIfPlayerIsLookingAtAngel`))))

(fn `DetectIfPlayerIsLookingAtAngel`
  (bind _returnvalue (`GameplayStatics.GetPlayerCameraManager` 0))
  (if (> (`KismetMathLibrary.Dot_VectorVector` (`KismetMathLibrary.GetForwardVector` (`KismetMathLibrary.FindLookAtRotation` (`self.K2_GetActorLocation` (`self.K2_GetPawn`)) (`self.K2_GetActorLocation` _returnvalue))) (`self.GetActorForwardVector` _returnvalue)) -0.5)
    (set `self.isLookingAtAngel` false)
    (`KismetSystemLibrary.PrintString` "Regarde plus l'ange" false)
    (`self.PursuitPlayer`)
    (else
      (set `self.isLookingAtAngel` true)
      (`KismetSystemLibrary.PrintString` "Regarde l'ange" false)
      (`self.StopMovement`))))

(fn `PursuitPlayer`
  (bind (_returnvalue_roll _returnvalue_pitch _returnvalue_yaw) (`KismetMathLibrary.BreakRotator` (`KismetMathLibrary.FindLookAtRotation` (`self.K2_GetActorLocation` (`self.K2_GetPawn`)) (`self.K2_GetActorLocation` (`GameplayStatics.GetPlayerCharacter` 0)))))
  (if (!= (`self.isLookingAtAngel`) true)
    (`self.K2_SetActorRotation` (`self.K2_GetPawn`) (`KismetMathLibrary.MakeRotator` 0.0 0.0 _returnvalue_yaw) false)
    (`self.MoveToActor` (`GameplayStatics.GetPlayerCharacter` 0) -1.0 false true true null)
    (else
      (`self.StopMovement`))))

(fn `UserConstructionScript`)