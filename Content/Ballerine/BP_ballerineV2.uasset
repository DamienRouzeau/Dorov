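; Ballerine actor (V2) that tracks its in and out presence timing and player outcomes through Blackboard values.
; Tick counts down InTimer while IsIn, otherwise OutTimer at a rate scaled by resolution, loose, AFK and hide multipliers.
; Despawn raises SurviveCount, KillPlayer lowers it, and Hide increments HidePerMinute.
; FinishScene saves and resets the scene timer, while SpawnInMap is an empty stub.
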(event `self.ReceiveTick`
  (params (DeltaSeconds :type "Float (single-precision)"))
  (bind _blackboard (`self.Blackboard`))
  (bind _blackboard_2 (`self.Blackboard`))
  (bind _blackboard_3 (`self.Blackboard`))
  (`parent.ReceiveTick` DeltaSeconds)
  (if (`self.IsIn`)
    (`BlackboardComponent.SetValueAsFloat` _blackboard_2 "InTimer" (- (`BlackboardComponent.GetValueAsFloat` _blackboard_2 "InTimer") DeltaSeconds))
    (else
      (`BlackboardComponent.SetValueAsFloat` _blackboard "OutTimer" (- (`BlackboardComponent.GetValueAsFloat` _blackboard "OutTimer") (* DeltaSeconds (`self.ResolutionMultiplier`) (`self.LooseMultiplicator`) (`self.AFKMultiplicator`) (`self.HideMultiplicator`))))
      (`BlackboardComponent.SetValueAsFloat` _blackboard_3 "OutTimer" (+ (`BlackboardComponent.GetValueAsFloat` _blackboard_3 "OutTimer") 0.0)))))

(event `FinishScene`
  (set `self.previousSceneTimer` (`self.currentSceneTimer`))
  (set `self.currentSceneTimer` 0.0))

(event `SpawnInMap`)

(event `Despawn`
  (bind _blackboard (`self.Blackboard`))
  (`BlackboardComponent.SetValueAsInt` _blackboard "SurviveCount" (+ (`BlackboardComponent.GetValueAsInt` _blackboard "SurviveCount") 1)))

(event `KillPlayer`
  (bind _blackboard (`self.Blackboard`))
  (`BlackboardComponent.SetValueAsInt` _blackboard "SurviveCount" (- (`BlackboardComponent.GetValueAsInt` _blackboard "SurviveCount") 1)))

(event `Hide`
  (bind _blackboard (`self.Blackboard`))
  (`BlackboardComponent.SetValueAsInt` _blackboard "HidePerMinute" (+ (`BlackboardComponent.GetValueAsInt` _blackboard "HidePerMinute") 1)))

(fn `UserConstructionScript`
  (`parent.UserConstructionScript`))