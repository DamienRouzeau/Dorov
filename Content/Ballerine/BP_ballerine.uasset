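; Ballerina enemy for a theater horror level that alternates between dancing to music under stage lights and hunting the player in the dark.
; Tick drives animation, footsteps and movement, while timers toggle music and lights, sending it back to its dance point or out to wander.
; AI perception starts a chase with music until distance breaks it.
; Phases alter speeds, timers and dances with blinking lights; death reloads the level.
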(event `ResetTimer`
  ;[1 1 1] Tick
  (goto _label :!via `Reset`))

(event `self.ReceiveTick`
  (params (DeltaSeconds :type "Float (single-precision)"))
  (bind _musicplayed (`self.MusicPlayed`))
  (bind _walksound (`self.WalkSound`))
  (bind _returnvalue (`self.K2_GetActorLocation` (`self.DancePoint`)))
  (bind _returnvalue_2 (`self.K2_GetActorLocation` (`self.As BP First Person Character`)))
  (bind _returnvalue_3 (== (`self.GetVelocity`) (0.0 0.0 0.0) :`ErrorTolerance` 0.1))
  (bind (_velocity_x _velocity_y _velocity_z) (`KismetMathLibrary.BreakVector` (`MovementComponent.Velocity` (`self.CharacterMovement`))))
  ;[1 1 1] Tick
  (if (not (`self.PlayerDead`))
    (if (or (> _velocity_x 0.0) (> _velocity_y 0.0) (> _velocity_z 0.0))
      (if (not (`AudioComponent.IsPlaying` _walksound))
        (`AudioComponent.Play` _walksound 0.0))
      (else
        (`AudioComponent.Stop` _walksound)))
    (if (and _returnvalue_3 _musicplayed)
      (`self.dance`)
      (elif (and _returnvalue_3 (not _musicplayed))
        (`self.idle`)
        (else
          (`self.walk`))))
    (if (`self.MusicPlayed`)
      (`AudioComponent.FadeOut` (`self.ChaseMusic`) 1.5 0.0 "Linear")
      (set `self.DarkTimerSet` false)
      (if (== (`self.K2_GetActorLocation`) _returnvalue :`ErrorTolerance` 1.0)
        (`/Engine/EditorBlueprintResources/StandardMacros.DoOnce` false :!label _label
          (:`Completed`
            (`self.SetTimerAndWait`)))
        (else
          (`|AIMoveTo` self _returnvalue (`self.DancePoint`) 10.0
            (:`OnSuccess`
              _)
            (:`OnFail`
              _))
          (`self.ResetWandering`)))
      (elif (`self.DarkTimerSet`)
        (`/Engine/EditorBlueprintResources/StandardMacros.IsValid` (`self.As BP First Person Character`)
          (:`Is Valid`
            (if (> (`KismetMathLibrary.Vector_Distance` _returnvalue_2 (`self.K2_GetActorLocation` self)) 1250.0)
              (`self.LooseChase`)))
          (:`Is Not Valid`
            _))
        (if (`self.isChasing`)
          (`|AIMoveTo` self _returnvalue_2 (`self.As BP First Person Character`) 2.0)
          (else
            (`/Engine/EditorBlueprintResources/StandardMacros.DoOnce` false :!label _label_2
              (:`Completed`
                (`|AIMoveTo` self (`self.K2_GetActorLocation` (`KismetArrayLibrary.Array_Random` (`self.PDI`))) null
                  (:`OnSuccess`
                    (`|AIMoveTo` self (`NavigationSystemV1.K2_GetRandomReachablePointInRadius` (`self.K2_GetActorLocation`) 2000.0 null null) null :!label _label_3
                      (:`OnSuccess`
                        (`KismetSystemLibrary.Delay` 0.5)
                        (goto _label_3)))))))))
        (else
          (set `self.DarkTimerSet` true)
          (`KismetSystemLibrary.K2_SetTimerDelegate` (delegate `SetTimerAndWait`) (`KismetMathLibrary.RandomFloatInRange` 20.0 50.0)))))))

(event `ResetWandering`
  ;[1 1 1] Tick
  (goto _label_2 :!via `Reset`))

(event `SetTimerAndWait`
  ;[1 1 1] BeginPlay
  (set `self.MusicPlayed` true)
  (if (== (`self.phase`) 1) :!label _label_4
    (set `self.timer` 600.0)
    (elif (== (`self.phase`) 2)
      (set `self.timer` 300.0)
      (else
        (set `self.timer` (`KismetMathLibrary.RandomFloatInRange` 35.0 50.0)))))
  (bind _returnvalue (`GameplayStatics.CreateSound2D` "/Game/Audio/Musics/Dorov_Glitched_Gloomy_Lake_V2.Dorov_Glitched_Gloomy_Lake_V2" 1.0 1.0 0.0 null false false :!label _label_5))
  (bind _output_get (set `self.Music` _returnvalue))
  (`AudioComponent.Play` _output_get 0.0)
  (for (_array_element _array_index) (`self.lights`)
    (`LightComponent.SetIntensity` (`Light.LightComponent` _array_element) (`|GetArrayItem` (`self.intensityLights`) _array_index)))
  (`self.SetActorHiddenInGame` false)
  (if (not (== (`self.phase`) 0))
    (`KismetSystemLibrary.K2_SetTimerDelegate` (delegate `StopMusic`) (`self.timer`))))

(event `ChangePhase`
  ;[1 1 1] BeginPlay
  (goto _label_4))

(event `self.ReceiveBeginPlay`
  ;[1 1 1] BeginPlay
  (for _array_element (`self.lights`)
    (`KismetArrayLibrary.Array_Add` (`self.intensityLights`) (`LightComponentBase.Intensity` (`Light.LightComponent` _array_element))))
  (bind _returnvalue (`GameplayStatics.CreateSound2D` "/Game/Audio/Sounds/SD_Bruit_de_pas_rapide_et_leger.SD_Bruit_de_pas_rapide_et_leger" 1.0 1.0 0.0 null false false))
  (set `self.WalkSound` _returnvalue)
  (bind _returnvalue_2 (`GameplayStatics.CreateSound2D` "/Game/Audio/Musics/Dorov_Chasse_v1.Dorov_Chasse_v1" 1.0 1.0 0.0 null false false))
  (set `self.ChaseMusic` _returnvalue_2)
  (goto _label_5))

(event `StopMusic`
  (bind _music (`self.Music`))
  ;[1 1 1] BeginPlay
  (set `self.objectsSet` 0)
  (set `self.MusicPlayed` false)
  (`/Engine/EditorBlueprintResources/StandardMacros.IsValid` _music
    (:`Is Valid`
      (`AudioComponent.Stop` _music)
      (for _array_element (`self.lights`)
        (`LightComponent.SetIntensity` (`Light.LightComponent` _array_element) 0.0))
      (`self.ResetTimer`))))

(event `checkChase`
  ;[1 0.33 0.7941] SpawnPoint
  (if (and (== (`self.phase`) 1) (>= (`self.objectsSet`) 2))
    (`self.K2_SetActorLocation` (`self.K2_GetActorLocation` (`KismetArrayLibrary.Array_Random` (`self.TPPoints`))) false true)
    (`self.StopMusic` :!label _label_6)
    (elif (and (== (`self.phase`) 2) (>= (`self.objectsSet`) 1))
      (goto _label_6))))

(event `dance`
  (bind _ballerine (`self.Ballerine`))
  (bind _phase (`self.phase`))
  ;[0.9011 0 1] Animations
  (`/Engine/EditorBlueprintResources/StandardMacros.DoOnce` false :!label _label_7
    (:`Completed`
      (if (== _phase 0)
        (`SkeletalMeshComponent.PlayAnimation` (`self.Ballerine`) "/Game/Ballerine/BallerineDeLucie/anims/DanceS1.DanceS1" true)
        (elif (== _phase 1)
          (`SkeletalMeshComponent.PlayAnimation` (`self.Ballerine`) "/Game/Ballerine/BallerineDeLucie/anims/DanceS2.DanceS2" true)
          (elif (== _phase 2)
            (`SkeletalMeshComponent.PlayAnimation` _ballerine "/Game/Ballerine/BallerineDeLucie/anims/DanceS3.DanceS3" true)
            (else
              (`SkeletalMeshComponent.PlayAnimation` _ballerine "/Game/Ballerine/BallerineDeLucie/anims/DanceS4.DanceS4" true)))))
      (`self.reset walk`)
      (`self.reset idle`))))

(event `reset dance`
  ;[0.9011 0 1] Animations
  (goto _label_7 :!via `Reset`))

(event `walk`
  ;[0.9011 0 1] Animations
  (`/Engine/EditorBlueprintResources/StandardMacros.DoOnce` false :!label _label_8
    (:`Completed`
      (`SkeletalMeshComponent.PlayAnimation` (`self.Ballerine`) "/Game/Ballerine/BallerineDeLucie/anims/Walking__3_.Walking__3_" true)
      (`self.reset dance`)
      (`self.reset idle`))))

(event `NewPhase`
  (bind _phase (`self.phase`))
  ;[1 0.114 0.114] NewPhase
  (if (not (>= _phase 3))
    (set `self.phase` (+ _phase 1)))
  (set `self.objectsSet` 0)
  (set `CharacterMovementComponent.MaxWalkSpeed` (`|GetArrayItem` (`self.speeds`) (`self.phase`)) (`self.CharacterMovement`))
  (`self.reset dance`)
  (`self.ChangePhase`)
  (`GameplayStatics.PlaySound2D` "/Game/Audio/Sounds/Clapping.Clapping" 1.0 1.0 0.0 null null)
  (for _array_element (`self.lights`) :!label _label_9
    (`LightComponent.SetLightColor` (`SpotLight.SpotLightComponent` _array_element) (struct :`R` 0.364583 :`G` 0.176595 :`B` 0.176595 :`A` 1.0) true))
  (`KismetSystemLibrary.K2_SetTimerDelegate` (delegate `LightToWhite`) (`self.BlinkSpeed`)))

(event `reset walk`
  ;[0.9011 0 1] Animations
  (goto _label_8 :!via `Reset`))

(event `LightToWhite`
  ;[1 0.114 0.114] NewPhase
  (for _array_element (`self.lights`)
    (`LightComponent.SetLightColor` (`SpotLight.SpotLightComponent` _array_element) (struct :`A` 1.0) true))
  (if (>= (`self.BlinkCount`) 13)
    (set `self.BlinkCount` 0)
    (for _array_element_2 (`self.lights`)
      (`LightComponent.SetLightColor` (`SpotLight.SpotLightComponent` _array_element_2) (struct :`R` 1.0 :`G` 1.0 :`B` 1.0 :`A` 1.0) true))
    (else
      (set `self.BlinkCount` (+ (`self.BlinkCount`) 1))
      (`KismetSystemLibrary.K2_SetTimerDelegate` (delegate `LightToGreen`) (`self.BlinkSpeed`)))))

(event `idle`
  ;[0.9011 0 1] Animations
  (`/Engine/EditorBlueprintResources/StandardMacros.DoOnce` false :!label _label_10
    (:`Completed`
      (`SkeletalMeshComponent.PlayAnimation` (`self.Ballerine`) "/Game/Ballerine/BallerineDeLucie/anims/Looking_Down.Looking_Down" true)
      (`self.reset dance`)
      (`self.reset walk`))))

(event `LightToGreen`
  ;[1 0.114 0.114] NewPhase
  (goto _label_9))

(event `reset idle`
  ;[0.9011 0 1] Animations
  (goto _label_10 :!via `Reset`))

(event `self.  deathArea.OnComponentBeginOverlap`
  (params (OverlappedComponent :type "PrimitiveComponent Object Reference") (OtherActor :type "Actor Object Reference") (OtherComp :type "PrimitiveComponent Object Reference") (OtherBodyIndex :type Integer) (bFromSweep :type Boolean) (SweepResult :type "HitResult Structure (by ref)"))
  ;[0 0 0] Death
  (bind _asbp_first_person_character (cast `/Game/FirstPerson/Blueprints/BP_FirstPersonCharacter` OtherActor))
  (`GameplayStatics.OpenLevelBySoftObjectPtr` "/Game/Maps/TheaterV2.TheaterV2" :!label _label_11))

(event `Dead`
  ;[0 0 0] Death
  (`/Game/FirstPerson/Blueprints/BP_FirstPersonCharacter.Die` (stale `self.  deathArea.OnComponentBeginOverlap` _asbp_first_person_character))
  (set `CharacterMovementComponent.MaxWalkSpeed` 0.0 (`self.CharacterMovement`))
  (bind (_returnvalue_roll _returnvalue_pitch _returnvalue_yaw) (`KismetMathLibrary.BreakRotator` (`self.K2_GetActorRotation` (stale `self.  deathArea.OnComponentBeginOverlap` _asbp_first_person_character))))
  ;;[1 1 1] Marche pas sans raison
  (`self.K2_SetActorLocationAndRotation` (+ (`self.K2_GetActorLocation` (stale `self.  deathArea.OnComponentBeginOverlap` _asbp_first_person_character)) (* (`self.GetActorForwardVector` (stale `self.  deathArea.OnComponentBeginOverlap` _asbp_first_person_character)) 7)) (`KismetMathLibrary.MakeRotator` _returnvalue_roll _returnvalue_pitch (* _returnvalue_yaw -1.0)))
  (set `self.PlayerDead` true)
  (`/Engine/EditorBlueprintResources/StandardMacros.DoOnce` false
    (:`Completed`
      (`SkeletalMeshComponent.PlayAnimation` (`self.Ch36_nonPBR`) "/Game/Ballerine/AnimationAndTextures/Zombie_Neck_Bite.Zombie_Neck_Bite" false)
      (`KismetSystemLibrary.Delay` 50.0)
      (goto _label_11))))

(event `self.AIPerception.OnTargetPerceptionUpdated`
  (params (Actor :type "Actor Object Reference") (Stimulus :type "AIStimulus Structure"))
  ;[0.074 1 0.243] DetectePlayer
  (bind _asbp_first_person_character (cast `/Game/FirstPerson/Blueprints/BP_FirstPersonCharacter` Actor))
  (if (and (not (`/Game/FirstPerson/Blueprints/BP_FirstPersonCharacter.IsInCloset` _asbp_first_person_character)) (not (`self.MusicPlayed`)))
    (set `self.As BP First Person Character` _asbp_first_person_character)
    (set `self.isChasing` true)
    (`/Engine/EditorBlueprintResources/StandardMacros.DoOnce` false :!label _label_12
      (:`Completed`
        (`AudioComponent.Play` (`self.ChaseMusic`) 0.9)
        (set `CharacterMovementComponent.MaxWalkSpeed` (`|GetArrayItem` (`self.runs`) (`self.phase`)) (`self.CharacterMovement`))))))

(event `LooseChase`
  ;[0 0.387 0.93] LooseChase
  (set `self.As BP First Person Character` null)
  (set `self.isChasing` false)
  (set `CharacterMovementComponent.MaxWalkSpeed` (`|GetArrayItem` (`self.runs`) (`self.phase`)) (`self.CharacterMovement`))
  (`/Engine/EditorBlueprintResources/StandardMacros.IsValid` (`self.ChaseMusic`)
    (:`Is Valid`
      (`KismetSystemLibrary.K2_SetTimerDelegate` (delegate `StopChaseMusic`) 2.2))
    (:`Is Not Valid`
      _))
  (`self.ResetWandering`))

(event `ResetChaseMusic`
  ;[0.074 1 0.243] DetectePlayer
  (goto _label_12 :!via `Reset`))

(event `StopChaseMusic`
  ;[0 0.387 0.93] LooseChase
  (if (not (`self.isChasing`))
    (`AudioComponent.FadeOut` (`self.ChaseMusic`) 1.5 0.0 "Linear")
    (`self.ResetChaseMusic`)))

(fn `UserConstructionScript`)